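; BP_LichEnemy is a melee Lich enemy that chases the player, attacks and takes damage.
; It moves toward the player after spawning; PawnSensing sets focus and chases the seen pawn, playing random left/right attack montages on a cooldown when close.
; A retriggerable delay clears sight and resumes GoToRandomLoc, which actually targets the player, as the random-point lookup is unused.
; Damage plays a hit reaction or, at zero health, disables collision and movement before despawning.
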(event OnSeePawn(PawnSensing)
  (params (Pawn :type Pawn%20Object%20Reference))
  (if (Variables|Default|GetAlive)
    (bind _output_get (Variables|Default|SetTargetPawn Pawn))
    (AI|SetFocus (AI|GetAIController (Pawn|GetController)) _output_get)
    (Utilities|FlowControl|Sequence
      (:then_0
        (Utilities|FlowControl|RetriggerableDelay 3.0)
        (Variables|Default|SetIsSeenPlayer? false)
        (CallFunction|GotoRandomLoc)
        (AI|ClearFocus (AI|GetAIController (Pawn|GetController))))
      (:then_1
        (Variables|Default|SetIsSeenPlayer? true)
        (AI|AIMoveTo self (Transformation|GetActorLocation (Variables|Default|GetTargetPawn)) 0 1e+02 false
          (:then
            (if (< (Math|Vector|Distance(Vector) (Transformation|GetActorLocation (Variables|Default|GetTargetPawn)) (Transformation|GetActorLocation)) 1.2e+02)
              (Utilities|FlowControl|Sequence :!label _label
                (:then_0
                  (Utilities|FlowControl|DoOnce false :!label _label_2
                    (:Completed
                      (Animation|PlayAnimMontage (.OutItem (Utilities|Array|Random (Utilities|Array|MakeArray "/Game/UndeadPack/Lich/Animations/Anim_Attack_Left_Montage.Anim_Attack_Left_Montage" "/Game/UndeadPack/Lich/Animations/Anim_Attack_Right_Montage.Anim_Attack_Right_Montage"))) 1.0 "None"))))
                (:then_1
                  (Utilities|FlowControl|Delay 2.0)
                  (goto _label_2 Reset)))))
          (:OnSuccess
            (goto _label)))))))

(event Custom|Go%20To%20Random%20Loc
  (if (Variables|Default|GetAlive)
    (if (not (Variables|Default|GetIsSeenPlayer?))
      (AI|AIMoveTo self "0, 0, 0" (Game|Player|GetPlayerPawn 0) 1e+02 false
        (:OnSuccess
          _)
        (:OnFail
          _))
      (Utilities|FlowControl|Delay 1.0)
      (if (not (Variables|Default|GetIsSeenPlayer?))
        (CallFunction|GotoRandomLoc)))))

(event EventBeginPlay
  (Utilities|FlowControl|Delay 2.0)
  (AI|AIMoveTo self "0, 0, 0" (Game|Player|GetPlayerPawn 0) 1e+02 false))

(event Game|Damage|EventAnyDamage
  (params (Damage :type Float%20%28single-precision%29) (DamageType :type Damage%20Type%20Object%20Reference) (InstigatedBy :type Controller%20Object%20Reference) (DamageCauser :type Actor%20Object%20Reference))
  (bind _output_get (Variables|Default|SetHealth (- (Variables|Default|GetHealth) Damage)))
  (if (<= _output_get 0.0)
    (Animation|StopAnimMontage (Animation|Montage|GetCurrentActiveMontage (Components|SkeletalMesh|GetAnimInstance (Variables|Character|GetMesh))))
    (Variables|Default|SetAlive false)
    (Collision|SetActorEnableCollision false)
    (Pawn|Components|CharacterMovement|SetMovementMode (Variables|Character|GetCharacterMovement) "MOVE_None" 0)
    (Actor|SetLifeSpan 1.0)
    (else
      (Animation|PlayAnimMontage "/Game/UndeadPack/Lich/Animations/Anim_Hit_Montage.Anim_Hit_Montage" 1.0 "None"))))

(fn ConstructionScript)