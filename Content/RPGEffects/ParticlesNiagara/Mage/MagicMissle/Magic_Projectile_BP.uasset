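; Mage magic missile projectile that damages what it hits and plays an impact effect before destroying itself.
; Overlapping an actor other than the Instigator, or the projectile stopping, runs a shared impact sequence.
; The sequence halts movement, swaps the Niagara system to the impact asset, fires a radial impulse, plays a sound and applies damage to the overlapped actor.
; A timeline drives the point light intensity, then destroys the actor when finished.
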(event OnProjectileStop(ProjectileMovement)
  (params (ImpactResult :type Hit%20Result%20Structure%20%28by%20ref%29))
  (bind _ns_mage_magicmissle (Variables|Default|GetNS_Mage_MagicMissle))
  (Utilities|FlowControl|Sequence
    (:then_0
      (Components|Movement|StopMovementImmediately (Variables|Default|GetProjectileMovement))
      (Class|NiagaraComponent|SetAsset _ns_mage_magicmissle "/Game/RPGEffects/ParticlesNiagara/Mage/MagicMissle/NS_Imact_Mage_MagicMissle.NS_Imact_Mage_MagicMissle" true)
      (Transformation|SetRelativeRotation _ns_mage_magicmissle "0.000000,180.000000,0.000000" false false)
      (Class|RadialForceComponent|FireImpulse (Variables|Default|GetRadialForce))
      (Audio|Components|Audio|Play (Variables|Default|GetCleaver_rSpark01_Cue) 0.0)
      (bind _a (Timeline|Timeline Play)
        (:Update
          (Rendering|Components|Light|SetIntensity (Variables|Default|GetPointLight) _a))
        (:Finished
          (Actor|DestroyActor))))
    (:then_1
      (Game|Damage|ApplyDamage (stale Collision|EventActorBeginOverlap OtherActor) (Variables|Default|GetBase%20Damage) 0 0))))

(event EventBeginPlay)

(event Collision|EventActorBeginOverlap
  (params (OtherActor :type Actor%20Object%20Reference))
  (bind _ns_mage_magicmissle (Variables|Default|GetNS_Mage_MagicMissle))
  (if (!= OtherActor (Variables|Actor|GetInstigator))
    (Utilities|FlowControl|Sequence
      (:then_0
        (Components|Movement|StopMovementImmediately (Variables|Default|GetProjectileMovement))
        (Class|NiagaraComponent|SetAsset _ns_mage_magicmissle "/Game/RPGEffects/ParticlesNiagara/Mage/MagicMissle/NS_Imact_Mage_MagicMissle.NS_Imact_Mage_MagicMissle" true)
        (Transformation|SetRelativeRotation _ns_mage_magicmissle "0.000000,180.000000,0.000000" false false)
        (Class|RadialForceComponent|FireImpulse (Variables|Default|GetRadialForce))
        (Audio|Components|Audio|Play (Variables|Default|GetCleaver_rSpark01_Cue) 0.0)
        (bind _a (Timeline|Timeline Play)
          (:Update
            (Rendering|Components|Light|SetIntensity (Variables|Default|GetPointLight) _a))
          (:Finished
            (Actor|DestroyActor))))
      (:then_1
        (Game|Damage|ApplyDamage OtherActor (Variables|Default|GetBase%20Damage) 0 0)))))

(fn ConstructionScript)