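; NPC character Blueprint that, once woken, walks off to a destination and removes itself from the level.
; Both wake-up events share one chain: set the Awake flag, wait a few seconds, then AI-move to TargetLocation, used as an offset from the actor's current position.
; The actor is destroyed only when the move succeeds.
; HasEnoughEnergy? is a stub that always returns false, and the construction script is empty.
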(event Custom|Call%20Wake%20Up%20NPC
  (Variables|Default|SetAwake true)
  (Utilities|FlowControl|Delay 6.0)
  (AI|AIMoveTo self (+ (Variables|Default|GetTargetLocation) (Transformation|GetActorLocation)) 0 1e+02 false
    (:OnSuccess
      (Actor|DestroyActor))))

(event EventWakeUpNPC
  (Variables|Default|SetAwake true)
  (Utilities|FlowControl|Delay 6.0)
  (AI|AIMoveTo self (+ (Variables|Default|GetTargetLocation) (Transformation|GetActorLocation)) 0 1e+02 false
    (:OnSuccess
      (Actor|DestroyActor))))

(fn ConstructionScript)

(fn HasEnoughEnergy?
  (params (Energy :type Float%20%28double-precision%29))
  (return false))