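; Player channelled Drain Health ability that fires a beam, damaging enemies and healing the caster by the same amount.
; Press retries casting on a timer until it starts; release or running out of mana plays the montage's End section.
; While active, Tick updates the beam, sphere-traces for a pawn and applies damage and cost scaled by delta time.
; Successful hits heal through the stats component and attach sparks; finishing clears effects and sound.
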(event Custom|DrainHealth
  (params (Amount :type Float%20%28double-precision%29))
  ;[0 0.272 1] Drain health
  (bind _statscomponent (Variables|Default|GetStatsComponent)
    (:then
      (Default|ModifyStat _statscomponent "(TagName=\"Stat.Health.Current\")" Amount))
    (:else)))

(event Custom|UpdateEffect
  ;[0 0.272 1] Update effect
  (bind _returnvalue (CallFunction|GetBeamTransform (Variables|Ability|Custom|GetDistance) (Variables|Ability|Custom|GetRadius) (CallFunction|GetSocketLocationonOwnerMesh (Variables|Default|GetBeamSocket)) (Variables|Ability|Custom|GetGoesThroughObjects)))
  (Variables|Default|SetEffectTransform _returnvalue)
  (Class|ParticleSystemComponent|SetBeamTargetPoint (Variables|Default|GetBeamParticle) 0 (CallFunction|GetEffectLocation)))

(event Custom|DestroyBeamParticle
  ;[0 0.272 1] Beam particle events
  (bind _beamparticle (Variables|Default|GetBeamParticle)
    (:then
      (Components|DestroyComponent _beamparticle))
    (:else)))

(event Custom|PlaySound
  ;[0 0.272 1] Sound
  (Variables|Default|GetSoundComponent
    (:then
      _)
    (:else
      (bind _returnvalue (Audio|SpawnSoundAttached (Variables|Ability|Custom|GetSound) (Variables|/Script/Engine.Character|GetMesh (Variables|Default|GetOwnerCharacter)) "None" "0, 0, 0" "0, 0, 0" "KeepRelativeOffset" false 1.0 1.0 0.0 0 0))
      (Variables|Default|SetSoundComponent _returnvalue)))
  (Audio|Components|Audio|FadeIn (Variables|Default|GetSoundComponent) 0.5 1.0 0.0 "Linear" :!class /Script/Engine.AudioComponent))

(event Custom|Loop_TryToStartAbility
  ;[0 0.272 1] On Pressed attempt to cast ability until it succeed or gets interrupted
  (CallFunction|TrytoStartAbility))

(event Custom|ClearTryToStartAbilityTimer
  ;[0 0.272 1] Clear Attempt To Cast Timer
  (Utilities|Time|ClearTimerbyFunctionName 0 "Loop_TryToStartAbility"))

(event Custom|StopSound
  ;[0 0.272 1] Sound
  (bind _soundcomponent (Variables|Default|GetSoundComponent)
    (:then
      (Audio|Components|Audio|FadeOut _soundcomponent 0.5 0.0 "Linear" :!class /Script/Engine.AudioComponent))
    (:else)))

(event Custom|DeactivateSparksParticle
  ;[0 0.272 1] Sparks particle
  (bind _sparksparticle (Variables|Default|GetSparksParticle)
    (:then
      (Components|Activation|Deactivate _sparksparticle))
    (:else)))

(event Custom|SpawnBeamParticle
  ;[0 0.272 1] Beam particle events
  (bind _returnvalue (Effects|SpawnEmitterAttached (Variables|Ability|Custom|GetDrainBeamParticle) (Variables|/Script/Engine.Character|GetMesh (Variables|Default|GetOwnerCharacter)) (Variables|Default|GetBeamSocket) "0, 0, 0" "0, 0, 0" "1.000000,1.000000,1.000000" "SnapToTarget"))
  (Variables|Default|SetBeamParticle _returnvalue))

(event Custom|UpdateSparksParticle
  (params (AttachToComponent :type Scene%20Component%20Object%20Reference))
  ;[0 0.272 1] Sparks particle
  (bind _sparksparticle (Variables|Default|GetSparksParticle)
    (:then
      (Components|Activation|Activate _sparksparticle false)
      (if (!= (Transformation|GetAttachParent _sparksparticle) AttachToComponent)
        (Transformation|AttachComponentToComponent (Variables|Default|GetSparksParticle) AttachToComponent "None" "SnapToTarget" "SnapToTarget" "SnapToTarget" true)))
    (:else
      (bind _returnvalue (Effects|SpawnEmitterAttached (Variables|Ability|Custom|GetDrainHitParticle) AttachToComponent "None" "0, 0, 0" "0, 0, 0" "1.000000,1.000000,1.000000" "SnapToTarget"))
      (Variables|Default|SetSparksParticle _returnvalue))))

(event EventdReleased
  ;[0 0.272 1] On released stop ability
  (CallFunction|ClearTrytoStartAbilityTimer)
  (if (Default|GetIsCasting (Variables|Default|GetAbilityComponent))
    (CallFunction|PlayAbilityMontage (CallFunction|GetAbilityMontage) "End" -1.0)
    (Default|FinishAbility (Variables|Default|GetAbilityComponent) "NewEnumerator0")))

(event EventdPressed
  ;[0 0.272 1] On Pressed attempt to cast ability until it succeed or gets interrupted
  (bind _result (CallFunction|TrytoStartAbility))
  (if (not _result)
    (Utilities|Time|SetTimerbyEvent (delegate Custom|Loop_TryToStartAbility) 0.1 true)))

(event EventTick
  (params (DeltaSeconds :type Float%20%28single-precision%29))
  ;[0 0.272 1] Event Tick
  (if (Variables|NonEdit|GetEffectEnabled)
    (CallFunction|UpdateEffect)
    (CallFunction|CheckforEnemies DeltaSeconds)
    (CallFunction|ApplyAbilityCost -1.0 DeltaSeconds)))

(event EventdSpawnEffect
  ;[0 0.272 1] Ability effect
  (Variables|NonEdit|SetEffectEnabled true)
  (CallFunction|SpawnBeamParticle)
  (CallFunction|UpdateEffect)
  (CallFunction|PlaySound))

(event EventdFinished
  (params (Result :type E_AbilityFinishResult%20Enum :default "NewEnumerator0"))
  ;[0 0.272 1] End of ability events
  (CallFunction|ClearTrytoStartAbilityTimer)
  (Variables|NonEdit|SetEffectEnabled false)
  (CallFunction|DestroyBeamParticle)
  (CallFunction|DeactivateSparksParticle)
  (CallFunction|StopSound)
  (switch Utilities|FlowControl|Switch|SwitchonE_AbilityFinishResult Result
    (:NewEnumerator3
      (CallFunction|PlayAbilityMontage (CallFunction|GetAbilityMontage) "End" -1.0))))

(event EventBeginPlay
  ;[0 0.272 1] Get owner's health component and store in variable
  (|CallParentFunction)
  (Variables|Default|SetStatsComponent (Actor|GetComponentbyClass (Components|GetOwner) "/Game/DynamicCombatSystem/DCS/Blueprints/Components/StatsManager/BP_StatsManagerComponent.BP_StatsManagerComponent_C")))

(fn ConstructionScript
  (|CallParentFunction))

(fn CheckforEnemies
  (params (DeltaTime :type Float%20%28double-precision%29))
  (bind _returnvalue (Components|GetOwner))
  (bind _returnvalue_2 (CallFunction|GetDamage DeltaTime))
  (bind (_outhit _returnvalue_3) (Collision|SphereTraceForObjects (CallFunction|GetSocketLocationonOwnerMesh (Variables|Default|GetBeamSocket)) (CallFunction|GetEffectLocation) (Variables|Ability|Custom|GetRadius) (Utilities|Array|MakeArray "ObjectTypeQuery3") false (Utilities|Array|MakeArray (Components|GetOwner)) "None"))
  (if _returnvalue_3
    (if (not (Utilities|Array|ContainsItem (LocalVariables|GetL_HitActors) (.HitActor (Collision|BreakHitResult _outhit))))
      (Utilities|Array|Add (LocalVariables|GetL_HitActors) (.HitActor (Collision|BreakHitResult _outhit)))
      (if (CallFunction|IsEnemy _returnvalue (.HitActor (Collision|BreakHitResult _outhit)))
        (bind _result (Class|ICanbeAttacked|TakeDamage(Message) (.HitActor (Collision|BreakHitResult _outhit)) (Utilities|Struct|MakeF_HitData _returnvalue_2 _returnvalue (Math|Vector|GetUnitDirection(Vector) (Transformation|GetActorLocation) (Transformation|GetActorLocation (.HitActor (Collision|BreakHitResult _outhit)))) _outhit "(GameplayTags=((TagName=\"HitData.CanBeBlocked\"),(TagName=\"HitData.DamageType.Magic\")))")))
        (if _result
          (CallFunction|DrainHealth _returnvalue_2)
          (CallFunction|UpdateSparksParticle (.HitComponent (Collision|BreakHitResult _outhit))))))
    (else
      (CallFunction|DeactivateSparksParticle))))

(fn TrytoStartAbility
  (bind _result (Default|StartCastingAbility (Variables|Default|GetAbilityComponent)))
  (if _result
    (CallFunction|PlayAbilityMontage (CallFunction|GetAbilityMontage) "None" -1.0)
    (CallFunction|ClearTrytoStartAbilityTimer)
    (return true)
    (else
      (return false))))