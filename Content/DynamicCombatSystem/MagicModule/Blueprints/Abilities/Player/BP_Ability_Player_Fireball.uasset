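; Player fireball ability for the Dynamic Combat System magic module that casts a montage on release and spawns a projectile.
; Repeated casts start with the first montage, then alternate between the next two, returning to the first after a retriggerable delay.
; The montage index selects the left or right hand socket for the spawn.
; The effect event aims the projectile by trace, spawns BP_MovingProjectile_Fireball with ability damage and applies the ability cost.
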(event Custom|ResetMontageCounter
  ;[0 0.272 1] When casted first, use montage at index 0 and then if keeps casting, use montages at indexes 1 & 2
  (Variables|NonEdit|SetMontageCounter 0))

(event Custom|UpdateMontageCounter
  ;[0 0.272 1] When casted first, use montage at index 0 and then if keeps casting, use montages at indexes 1 & 2
  (bind _result (Math|Integer|IncrementInt (Variables|NonEdit|GetMontageCounter))
    (:%20%20
      (if (> _result (Utilities|Array|LastIndex (Variables|Default|GetAbilityMontages)))
        (Variables|NonEdit|SetMontageCounter 1)))))

(event Custom|UpdateSocket
  ;[0 0.272 1] Use left hand socket only for 1st index because animation at this index uses left hand
  (switch int (Variables|NonEdit|GetMontageCounter)
    (:0
      (Variables|NonEdit|SetUseLeftHandSocket false))
    (:1
      (Variables|NonEdit|SetUseLeftHandSocket true))
    (:2
      (Variables|NonEdit|SetUseLeftHandSocket false))))

(event EventdReleased
  (bind _result (Default|StartCastingAbility (Variables|Default|GetAbilityComponent)))
  (if _result
    (CallFunction|UpdateSocket)
    (bind _duration (CallFunction|PlayAbilityMontage (CallFunction|GetAbilityMontage (Variables|NonEdit|GetMontageCounter)) "None" -1.0))
    ;[0 0.272 1] Handle montage counter
    (CallFunction|UpdateMontageCounter)
    (Utilities|FlowControl|RetriggerableDelay _duration)
    (CallFunction|ResetMontageCounter)))

(event EventdSpawnEffect
  (bind _returnvalue (Components|GetOwner))
  ;[0 0.272 1] Spawn Fireball projectile and consume mana
  (bind _returnvalue_2 (CallFunction|GetProjectileTransform (CallFunction|GetSocketLocationonOwnerMesh (select (Variables|NonEdit|GetUseLeftHandSocket) (Variables|Default|GetLeftHandSocket) (Variables|Default|GetRightHandSocket))) 1.0 1.5e+04))
  (bind _output_get (Variables|Default|SetEffectTransform _returnvalue_2))
  (Game|SpawnActorfromClass "/Game/DynamicCombatSystem/MagicModule/Blueprints/Projectiles/Instances/BP_MovingProjectile_Fireball.BP_MovingProjectile_Fireball_C" _output_get "AdjustIfPossibleButAlwaysSpawn" "OverrideRootScale" _returnvalue (CallFunction|GetDamage 1.0) 3.5e+03 1e+04 true (Game|GetInstigator _returnvalue))
  (CallFunction|ApplyAbilityCost -1.0 1.0))

(fn ConstructionScript
  (|CallParentFunction))