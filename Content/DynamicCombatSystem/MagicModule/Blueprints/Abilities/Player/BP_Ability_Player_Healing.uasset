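; Player magic ability that channels healing on the caster for as long as the input is held.
; Pressing retries casting on a looping timer until it starts, and releasing plays the montage's End section and finishes the ability.
; While the effect is enabled, Tick restores health through the stats component and drains ability cost, both scaled by delta time.
; Attached particle and sound components are reused across casts and stopped when the ability finishes.
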(event Custom|Heal
  (params (Amount :type Float%20%28double-precision%29))
  ;[0 0.272 1] Heal event
  (bind _statscomponent (Variables|Default|GetStatsComponent)
    (:then
      (Default|ModifyStat _statscomponent "(TagName=\"Stat.Health.Current\")" Amount))
    (:else)))

(event Custom|SpawnParticle
  ;[0 0.272 1] Particle events
  (bind _particle (Variables|Components|GetParticle)
    (:then
      (Components|Activation|Activate _particle false))
    (:else
      (bind _returnvalue (Effects|SpawnEmitterAttached (Variables|Ability|Custom|GetHealingParticle) (Variables|/Script/Engine.Character|GetMesh (Variables|Default|GetOwnerCharacter)) "None" "0, 0,100.000000"))
      (Variables|Components|SetParticle _returnvalue))))

(event Custom|DeactivateParticle
  ;[0 0.272 1] Particle events
  (bind _particle (Variables|Components|GetParticle)
    (:then
      (Components|Activation|Deactivate _particle))
    (:else)))

(event Custom|PlaySound
  ;[0 0.272 1] Sound
  (Variables|Default|GetSoundComponent
    (:then
      _)
    (:else
      (bind _returnvalue (Audio|SpawnSoundAttached (Variables|Ability|Custom|GetSound) (Variables|/Script/Engine.Character|GetMesh (Variables|Default|GetOwnerCharacter)) "None" "0, 0, 0" "0, 0, 0" "KeepRelativeOffset" false 1.0 1.0 0.0 0 0))
      (Variables|Default|SetSoundComponent _returnvalue)))
  (Audio|Components|Audio|FadeIn (Variables|Default|GetSoundComponent) 0.5 1.0 0.0 "Linear" :!class /Script/Engine.AudioComponent))

(event Custom|Loop_TryToStartAbility
  ;[0 0.272 1] On Pressed attempt to cast ability until it succeed or gets interrupted
  (CallFunction|TrytoStartAbility))

(event Custom|ClearTryToStartAbilityTimer
  ;[0 0.272 1] Clear Attempt To Cast Timer
  (Utilities|Time|ClearTimerbyFunctionName 0 "Loop_TryToStartAbility"))

(event Custom|StopSound
  ;[0 0.272 1] Sound
  (bind _soundcomponent (Variables|Default|GetSoundComponent)
    (:then
      (Audio|Components|Audio|FadeOut _soundcomponent 0.5 0.0 "Linear" :!class /Script/Engine.AudioComponent))
    (:else)))

(event EventdReleased
  ;[0 0.272 1] On released stop ability
  (CallFunction|ClearTrytoStartAbilityTimer)
  (if (Default|GetIsCasting (Variables|Default|GetAbilityComponent))
    (CallFunction|PlayAbilityMontage (CallFunction|GetAbilityMontage) "End" -1.0)
    (Default|FinishAbility (Variables|Default|GetAbilityComponent) "NewEnumerator0")))

(event EventdPressed
  ;[0 0.272 1] On Pressed attempt to cast ability until it succeed or gets interrupted
  (bind _result (CallFunction|TrytoStartAbility))
  (if (not _result)
    (Utilities|Time|SetTimerbyEvent (delegate Custom|Loop_TryToStartAbility) 0.1 true)))

(event EventTick
  (params (DeltaSeconds :type Float%20%28single-precision%29))
  ;[0 0.272 1] Keep healing and consuming mana while effect is enabled
  (if (Variables|NonEdit|GetEffectEnabled)
    (CallFunction|Heal (* (Variables|Ability|Custom|GetHealAmount) DeltaSeconds))
    (CallFunction|ApplyAbilityCost -1.0 DeltaSeconds)))

(event EventdSpawnEffect
  ;[0 0.272 1] Ability effect
  (Variables|NonEdit|SetEffectEnabled true)
  (CallFunction|SpawnParticle)
  (CallFunction|PlaySound))

(event EventdFinished
  (params (Result :type E_AbilityFinishResult%20Enum :default "NewEnumerator0"))
  ;[0 0.272 1] End of ability events
  (CallFunction|ClearTrytoStartAbilityTimer)
  (Variables|NonEdit|SetEffectEnabled false)
  (CallFunction|DeactivateParticle)
  (CallFunction|StopSound)
  (switch Utilities|FlowControl|Switch|SwitchonE_AbilityFinishResult Result
    (:NewEnumerator3
      (CallFunction|PlayAbilityMontage (CallFunction|GetAbilityMontage) "End" -1.0))))

(event EventBeginPlay
  ;[0 0.272 1] Get owner's health component and store in variable
  (|CallParentFunction)
  (Variables|Default|SetStatsComponent (Actor|GetComponentbyClass (Components|GetOwner) "/Game/DynamicCombatSystem/DCS/Blueprints/Components/StatsManager/BP_StatsManagerComponent.BP_StatsManagerComponent_C")))

(fn ConstructionScript
  (|CallParentFunction))

(fn TrytoStartAbility
  (bind _result (Default|StartCastingAbility (Variables|Default|GetAbilityComponent)))
  (if _result
    (CallFunction|PlayAbilityMontage (CallFunction|GetAbilityMontage) "None" -1.0)
    (CallFunction|ClearTrytoStartAbilityTimer)
    (return true)
    (else
      (return false))))