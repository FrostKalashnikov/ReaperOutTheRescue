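; Player channeled magic ability that creates a damaging vortex, which drifts at constant speed toward the targeted surface point.
; Pressing shows the indicator and retries casting on a timer until it starts, while releasing stops the timer and finishes any active cast.
; Once spawned, the effect charges an initial cost, then each tick moves particle and sound, capsule-traces to damage enemies, and drains mana, both scaled by delta time.
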(event Custom|SpawnParticle
  ;[0 0.272 1] Vortex Particle
  (bind _particlecomponent (Variables|Default|GetParticleComponent)
    (:then
      (Components|Activation|Activate _particlecomponent false)
      (Transformation|SetWorldLocation _particlecomponent (Variables|NonEdit|GetVortexLocation) false false))
    (:else
      (bind _returnvalue (Effects|SpawnEmitteratLocation (Variables|Ability|Custom|GetVortexParticle) (Variables|NonEdit|GetVortexLocation)))
      (Variables|Default|SetParticleComponent _returnvalue))))

(event Custom|DeactivateParticle
  ;[0 0.272 1] Vortex Particle
  (bind _particlecomponent (Variables|Default|GetParticleComponent)
    (:then
      (Components|Activation|Deactivate _particlecomponent))
    (:else)))

(event Custom|PlaySound
  ;[0 0.272 1] Sound
  (bind _soundcomponent (Variables|Default|GetSoundComponent)
    (:then
      (Transformation|SetWorldLocation _soundcomponent (Variables|NonEdit|GetVortexLocation) false false))
    (:else
      (bind _returnvalue (Audio|SpawnSoundatLocation (Variables|Ability|Custom|GetSound) (Variables|NonEdit|GetVortexLocation) "0, 0, 0" 1.0 1.0 0.0 0 0))
      (Variables|Default|SetSoundComponent _returnvalue)))
  (Audio|Components|Audio|FadeIn (Variables|Default|GetSoundComponent) 0.5 1.0 0.0 "Linear" :!class /Script/Engine.AudioComponent))

(event Custom|Loop_TryToStartAbility
  ;[0 0.272 1] On Pressed attempt to cast ability until it succeed or gets interrupted
  (CallFunction|TrytoStartAbility))

(event Custom|ClearTryToStartAbilityTimer
  ;[0 0.272 1] Clear Attempt To Cast Timer
  (Utilities|Time|ClearTimerbyFunctionName 0 "Loop_TryToStartAbility"))

(event Custom|StopSound
  ;[0 0.272 1] Sound
  (bind _soundcomponent (Variables|Default|GetSoundComponent)
    (:then
      (Audio|Components|Audio|FadeOut _soundcomponent 0.5 0.0 "Linear" :!class /Script/Engine.AudioComponent))
    (:else)))

(event Custom|UpdateVortex
  ;[0 0.272 1] Update vortex location, then location of particle & sound
  (Variables|NonEdit|SetVortexLocation (Math|Interpolation|VInterptoConstant (Variables|NonEdit|GetVortexLocation) (CallFunction|GetEffectLocation) (Utilities|Time|GetWorldDeltaSeconds) (Variables|Ability|Custom|GetVortexSpeed)))
  (Utilities|FlowControl|Sequence
    (:then_0
      (bind _particlecomponent (Variables|Default|GetParticleComponent)
        (:then
          (Transformation|SetWorldLocationAndRotation _particlecomponent (Variables|NonEdit|GetVortexLocation) "0, 0, 0" false false))
        (:else)))
    (:then_1
      (bind _soundcomponent (Variables|Default|GetSoundComponent)
        (:then
          (Transformation|SetWorldLocation _soundcomponent (Variables|NonEdit|GetVortexLocation) false false))
        (:else)))))

(event EventdPressed
  ;[0 0.272 1] On Pressed attempt to cast ability until it succeed or gets interrupted
  (CallFunction|ShowIndicator (CallFunction|GetEffectLocation))
  (bind _result (CallFunction|TrytoStartAbility))
  (if (not _result)
    (Utilities|Time|SetTimerbyEvent (delegate Custom|Loop_TryToStartAbility) 0.1 true)))

(event EventTick
  (params (DeltaSeconds :type Float%20%28single-precision%29))
  ;[0 0.272 1] Tick, update effect transform, spell indicator, check for enemies and cosume mana
  (Utilities|FlowControl|Sequence
    (:then_0
      (if (Default|IsUsingAbility (Variables|Default|GetAbilityComponent))
        (bind _transform (CallFunction|GetSurfaceTransform (Variables|Ability|Custom|GetRange) (Variables|Ability|Custom|GetMaxSurfaceAngle) 2e+03))
        (Variables|Default|SetEffectTransform _transform)
        (Default|UpdateSpellIndicatorLocation (Variables|Default|GetAbilityComponent) (CallFunction|GetEffectLocation))))
    (:then_1
      (if (Variables|NonEdit|GetEffectEnabled)
        (CallFunction|UpdateVortex)
        (CallFunction|CheckforEnemies DeltaSeconds)
        (CallFunction|ApplyAbilityCost -1.0 DeltaSeconds)))))

(event EventdSpawnEffect
  ;[0 0.272 1] Effect
  (Variables|NonEdit|SetEffectEnabled true)
  (Variables|NonEdit|SetVortexLocation (CallFunction|GetEffectLocation))
  (CallFunction|PlaySound)
  (CallFunction|SpawnParticle)
  (CallFunction|ApplyAbilityCost (Variables|Ability|Custom|GetInitialUseAbilityCost) 1.0))

(event EventdFinished
  (params (Result :type E_AbilityFinishResult%20Enum :default "NewEnumerator0"))
  ;[0 0.272 1] End of ability events
  (CallFunction|ClearTrytoStartAbilityTimer)
  (Variables|NonEdit|SetEffectEnabled false)
  (CallFunction|DeactivateParticle)
  (CallFunction|StopSound)
  (switch Utilities|FlowControl|Switch|SwitchonE_AbilityFinishResult Result
    (:NewEnumerator3
      (CallFunction|PlayAbilityMontage (CallFunction|GetAbilityMontage) "End" -1.0))))

(event EventdReleased
  ;[0 0.272 1] On released stop ability
  (CallFunction|ClearTrytoStartAbilityTimer)
  (if (Default|GetIsCasting (Variables|Default|GetAbilityComponent))
    (CallFunction|PlayAbilityMontage (CallFunction|GetAbilityMontage) "End" -1.0)
    (Default|FinishAbility (Variables|Default|GetAbilityComponent) "NewEnumerator0")))

(fn ConstructionScript
  (|CallParentFunction))

(fn CheckforEnemies
  (params (DeltaTime :type Float%20%28double-precision%29))
  (bind _returnvalue (Components|GetOwner))
  (bind _collisionheight (Variables|Ability|Custom|GetCollisionHeight))
  (bind _particlecomponent (Variables|Default|GetParticleComponent))
  (bind _returnvalue_2 (Transformation|GetWorldLocation _particlecomponent))
  (bind (_x _y _z) (Math|Vector|BreakVector _returnvalue_2))
  (bind _returnvalue_3 (+ _z _collisionheight))
  (bind _returnvalue_4 (Math|Vector|MakeVector _x _y _returnvalue_3))
  (bind _outhits (Class|KismetSystemLibrary|CapsuleTraceMultiforObjects _returnvalue_4 (+ _returnvalue_4 "0, 0,1.000000") (Variables|Ability|Custom|GetRadius) (Variables|Ability|Custom|GetCollisionHeight) (Utilities|Array|MakeArray "ObjectTypeQuery3") false (Utilities|Array|MakeArray (Components|GetOwner)) "None" true))
  (for _array_element _outhits
    (if (not (Utilities|Array|ContainsItem (LocalVariables|GetL_HitActors) (.HitActor (Collision|BreakHitResult _array_element))))
      (Utilities|Array|Add (LocalVariables|GetL_HitActors) (.HitActor (Collision|BreakHitResult _array_element)))
      (if (CallFunction|IsEnemy _returnvalue (.HitActor (Collision|BreakHitResult _array_element)))
        (Class|ICanbeAttacked|TakeDamage(Message) (.HitActor (Collision|BreakHitResult _array_element)) (Utilities|Struct|MakeF_HitData (CallFunction|GetDamage DeltaTime) _returnvalue (Math|Vector|GetUnitDirection(Vector) (Transformation|GetActorLocation) (Transformation|GetActorLocation (.HitActor (Collision|BreakHitResult _array_element)))) _array_element "(GameplayTags=((TagName=\"HitData.DamageType.Magic\")))"))))))

(fn TrytoStartAbility
  (bind _result (Default|StartCastingAbility (Variables|Default|GetAbilityComponent)))
  (if _result
    (CallFunction|PlayAbilityMontage (CallFunction|GetAbilityMontage) "None" -1.0)
    (CallFunction|ClearTrytoStartAbilityTimer)
    (return true)
    (else
      (return false))))