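; Player channeled lightning sparks ability that fires a beam from a mesh socket, damaging enemies along it while held.
; Press retries casting on a timer until it succeeds; release plays the montage's End section and finishes the ability.
; While the effect runs, Tick re-aims the particle beam, sphere-traces pawns for blockable, delta-time-scaled damage once per actor, and drains cost.
; Finishing removes the particle and fades out the sound.
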(event Custom|SpawnParticle
  ;[0 0.272 1] Spawn particle and update it's target point immediately
  (bind _returnvalue (Effects|SpawnEmitterAttached (Variables|Ability|Custom|GetBeamParticle) (Variables|/Script/Engine.Character|GetMesh (Variables|Default|GetOwnerCharacter)) (Variables|Default|GetBeamSocket) "0, 0, 0" "0, 0, 0" "1.000000,1.000000,1.000000" "SnapToTarget"))
  (Variables|Default|SetParticle _returnvalue))

(event Custom|UpdateEffect
  ;[0 0.272 1] Update effect
  (bind _returnvalue (CallFunction|GetBeamTransform (Variables|Ability|Custom|GetDistance) (Variables|Ability|Custom|GetRadius) (CallFunction|GetSocketLocationonOwnerMesh (Variables|Default|GetBeamSocket)) (Variables|Ability|Custom|GetGoesThroughObjects)))
  (Variables|Default|SetEffectTransform _returnvalue)
  (Class|ParticleSystemComponent|SetBeamTargetPoint (Variables|Default|GetParticle) 0 (CallFunction|GetEffectLocation)))

(event Custom|DestroyParticle
  ;[0 0.272 1] Destroy prticle
  (bind _particle (Variables|Default|GetParticle)
    (:then
      (Components|DestroyComponent _particle))
    (:else)))

(event Custom|PlaySound
  ;[0 0.272 1] Sound
  (Variables|Default|GetSoundComponent
    (:then
      _)
    (:else
      (bind _returnvalue (Audio|SpawnSoundAttached (Variables|Ability|Custom|GetSound) (Variables|/Script/Engine.Character|GetMesh (Variables|Default|GetOwnerCharacter)) "None" "0, 0, 0" "0, 0, 0" "KeepRelativeOffset" false 1.0 1.0 0.0 0 0))
      (Variables|Default|SetSoundComponent _returnvalue)))
  (Audio|Components|Audio|FadeIn (Variables|Default|GetSoundComponent) 0.5 1.0 0.0 "Linear" :!class /Script/Engine.AudioComponent))

(event Custom|Loop_TryToStartAbility
  ;[0 0.272 1] On Pressed attempt to cast ability until it succeed or gets interrupted
  (CallFunction|TrytoStartAbility))

(event Custom|ClearTryToStartAbilityTimer
  ;[0 0.272 1] Clear Attempt To Cast Timer
  (Utilities|Time|ClearTimerbyFunctionName 0 "Loop_TryToStartAbility"))

(event Custom|StopSound
  ;[0 0.272 1] Sound
  (bind _soundcomponent (Variables|Default|GetSoundComponent)
    (:then
      (Audio|Components|Audio|FadeOut _soundcomponent 0.5 0.0 "Linear" :!class /Script/Engine.AudioComponent))
    (:else)))

(event EventdReleased
  ;[0 0.272 1] On released stop ability
  (CallFunction|ClearTrytoStartAbilityTimer)
  (if (Default|GetIsCasting (Variables|Default|GetAbilityComponent))
    (CallFunction|PlayAbilityMontage (CallFunction|GetAbilityMontage) "End" -1.0)
    (Default|FinishAbility (Variables|Default|GetAbilityComponent) "NewEnumerator0")))

(event EventdPressed
  ;[0 0.272 1] On Pressed attempt to cast ability until it succeed or gets interrupted
  (bind _result (CallFunction|TrytoStartAbility))
  (if (not _result)
    (Utilities|Time|SetTimerbyEvent (delegate Custom|Loop_TryToStartAbility) 0.1 true)))

(event EventTick
  (params (DeltaSeconds :type Float%20%28single-precision%29))
  ;[0 0.272 1] On Tick update effect transform, check for enemies and consume mana
  (if (Variables|NonEdit|GetEffectEnabled)
    (CallFunction|UpdateEffect)
    (CallFunction|CheckforEnemies DeltaSeconds)
    (CallFunction|ApplyAbilityCost -1.0 DeltaSeconds)))

(event EventdSpawnEffect
  ;[0 0.272 1] Ability Effect
  (Variables|NonEdit|SetEffectEnabled true)
  (CallFunction|SpawnParticle)
  (CallFunction|UpdateEffect)
  (CallFunction|PlaySound))

(event EventdFinished
  (params (Result :type E_AbilityFinishResult%20Enum :default "NewEnumerator0"))
  ;[0 0.272 1] End of ability
  (CallFunction|ClearTrytoStartAbilityTimer)
  (Variables|NonEdit|SetEffectEnabled false)
  (CallFunction|DestroyParticle)
  (CallFunction|StopSound)
  (switch Utilities|FlowControl|Switch|SwitchonE_AbilityFinishResult Result
    (:NewEnumerator3
      (CallFunction|PlayAbilityMontage (CallFunction|GetAbilityMontage) "End" -1.0))))

(fn ConstructionScript
  (|CallParentFunction))

(fn CheckforEnemies
  (params (DeltaTime :type Float%20%28double-precision%29))
  (bind _returnvalue (Components|GetOwner))
  (bind _outhits (Collision|MultiSphereTraceForObjects (CallFunction|GetSocketLocationonOwnerMesh (Variables|Default|GetBeamSocket)) (CallFunction|GetEffectLocation) (Variables|Ability|Custom|GetRadius) (Utilities|Array|MakeArray "ObjectTypeQuery3") false (Utilities|Array|MakeArray (Components|GetOwner)) "None"))
  (for _array_element _outhits
    (bind _output_get (LocalVariables|SetL_HitActor (.HitActor (Collision|BreakHitResult _array_element))))
    (if (not (Utilities|Array|ContainsItem (LocalVariables|GetL_HitActors) _output_get))
      (Utilities|Array|Add (LocalVariables|GetL_HitActors) (LocalVariables|GetL_HitActor))
      (if (CallFunction|IsEnemy _returnvalue (.HitActor (Collision|BreakHitResult _array_element)))
        (Class|ICanbeAttacked|TakeDamage(Message) (LocalVariables|GetL_HitActor) (Utilities|Struct|MakeF_HitData (CallFunction|GetDamage DeltaTime) _returnvalue (Math|Vector|GetUnitDirection(Vector) (Transformation|GetActorLocation _returnvalue) (Transformation|GetActorLocation (LocalVariables|GetL_HitActor))) _array_element "(GameplayTags=((TagName=\"HitData.CanBeBlocked\"),(TagName=\"HitData.DamageType.Magic\")))"))))))

(fn TrytoStartAbility
  (bind _result (Default|StartCastingAbility (Variables|Default|GetAbilityComponent)))
  (if _result
    (CallFunction|PlayAbilityMontage (CallFunction|GetAbilityMontage) "None" -1.0)
    (CallFunction|ClearTrytoStartAbilityTimer)
    (return true)
    (else
      (return false))))