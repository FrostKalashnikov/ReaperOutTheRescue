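; Player ability in the magic module that lets the player aim and place a damage trap on a surface.
; While pressed and not casting, Tick updates the effect transform from a surface query limited by range, angle and height deviation, moving the indicator with it.
; Release starts the cast montage, or hides the indicator if no cast is running.
; The spawn-effect event spawns BP_AE_DamageTrap at that transform, applies the ability cost and plays a sound.
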(event Custom|PlaySound
  ;[0 0.272 1] Play Sound
  (Audio|PlaySoundatLocation (Variables|Ability|Custom|GetSound) (CallFunction|GetEffectLocation) "0, 0, 0" 1.0 1.0 0.0 0 0 0 0))

(event Custom|UpdateEffect
  ;[0 0.272 1] Update effect transform and it's indicator
  (bind _transform (CallFunction|GetSurfaceTransform (Variables|Ability|Custom|GetRange) (Variables|Ability|Custom|GetMaxSurfaceAngle) (Variables|Ability|Custom|GetMaxHeightDeviation)))
  (Variables|Default|SetEffectTransform _transform)
  (CallFunction|UpdateIndicator (CallFunction|GetEffectLocation)))

(event EventdReleased
  ;[0 0.272 1] On Ability released cast ability or hide spell indicator if not casting
  (bind _result (Default|StartCastingAbility (Variables|Default|GetAbilityComponent)))
  (if _result
    (CallFunction|PlayAbilityMontage (CallFunction|GetAbilityMontage) "None" -1.0)
    (CallFunction|UpdateEffect)
    (elif (not (Default|GetIsCasting (Variables|Default|GetAbilityComponent)))
      (CallFunction|HideIndicator))))

(event EventdPressed
  ;[0 0.272 1] On Ability pressed show spell indicator
  (if (not (Default|GetIsCasting (Variables|Default|GetAbilityComponent)))
    (CallFunction|UpdateEffect)
    (CallFunction|ShowIndicator (CallFunction|GetEffectLocation))))

(event EventTick
  (params (DeltaSeconds :type Float%20%28single-precision%29))
  (bind _abilitycomponent (Variables|Default|GetAbilityComponent))
  ;[0 0.272 1] Update effect transform only if ability is pressed but not already casting
  (if (and (Default|GetIsPressed _abilitycomponent) (not (Default|GetIsCasting _abilitycomponent)))
    (CallFunction|UpdateEffect)))

(event EventdSpawnEffect
  (bind _returnvalue (Components|GetOwner))
  ;[0 0.272 1] Effect
  (Game|SpawnActorfromClass "/Game/DynamicCombatSystem/DCS/Blueprints/Components/Ability/AbilityEffects/BP_AE_DamageTrap.BP_AE_DamageTrap_C" (Variables|Default|GetEffectTransform) "AlwaysSpawn" "OverrideRootScale" _returnvalue (Variables|Ability|Custom|GetTrapRadius) (Variables|Ability|Custom|GetDamageRadius) (CallFunction|GetDamage 1.0) (Variables|Ability|Custom|GetDuration) (Variables|Ability|Custom|GetActivationDelay) "None" (Game|GetInstigator _returnvalue))
  (CallFunction|ApplyAbilityCost -1.0 1.0)
  (CallFunction|PlaySound))

(fn ConstructionScript
  (|CallParentFunction))