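; AI ability in the Dynamic Combat System magic module that summons a temporary minion against the caster's target.
; On release, an EQS query picks a summon spot, which is snapped to the ground before the casting montage plays, or the ability finishes on failure.
; The effect spawns the minion facing the target, assigns its target, plays a sound and applies cost.
; A timed IsMarkedToKill activity limits the minion's lifetime.
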(event Custom|OnQueryFinishedEvent
  (params (QueryInstance :type Env%20Query%20Instance%20Blueprint%20Wrapper%20Object%20Reference) (QueryStatus :type EEnvQueryStatus%20Enum :default "Processing"))
  ;[0 0.272 1] When EQS query finish, save teleport location in EffectTransform variable and play anim montage
  (bind (_resultlocations _returnvalue) (AI|EQS|GetQueryResultsasLocations QueryInstance))
  (if _returnvalue
    (bind (_groundlocation _normal _result) (CallFunction|FindGroundLocation (Utilities|Array|Get(acopy) _resultlocations) 8e+01))
    (if _result
      (Variables|Default|SetEffectTransform (Math|Transform|MakeTransform _groundlocation (Math|Conversions|RotationFromXVector (Math|Vector|GetUnitDirection(Vector) (Transformation|GetActorLocation (Components|GetOwner)) _groundlocation))))
      (CallFunction|PlayAbilityMontage (CallFunction|GetAbilityMontage) "None" -1.0)
      (else
        (Default|FinishAbility (Variables|Default|GetAbilityComponent) "NewEnumerator1" :!label _label)))
    (else
      (goto _label))))

(event Custom|PlaySound
  ;[0 0.272 1] Play Sound
  (Audio|PlaySoundatLocation (Variables|Ability|Custom|GetSound) (CallFunction|GetEffectLocation) "0, 0, 0" 1.0 1.0 0.0 0 0 0 0))

(event EventdReleased
  ;[0 0.272 1] On Pressed check whether ability can be started
  (bind _result (Default|StartCastingAbility (Variables|Default|GetAbilityComponent)))
  (if _result
    ;[0 0.272 1] Run EQS Query to find teleport location
    (bind _returnvalue (AI|EQS|RunEQSQuery "/Game/DynamicCombatSystem/MagicModule/Blueprints/AI/EQS/EQS_SummonSpot.EQS_SummonSpot" (Components|GetOwner) "RandomBest25Pct"))
    (EventDispatchers|AssignOnQueryFinishedEvent _returnvalue (EventDispatchers|CreateEvent :!event Custom|OnQueryFinishedEvent))))

(event EventdSpawnEffect
  ;[0 0.272 1] On ability effect teleport character
  (CallFunction|SummonMinion)
  (CallFunction|PlaySound)
  (CallFunction|ApplyAbilityCost -1.0 1.0))

(fn ConstructionScript
  (|CallParentFunction))

(fn SummonMinion
  (bind _returnvalue (Game|SpawnActorfromClass (Variables|Ability|Custom|GetAIClassToSpawn) (Math|Transform|MakeTransform (CallFunction|GetEffectLocation) (Math|Rotator|MakeRotator 0.0 0.0 (.Yaw (Math|Rotator|BreakRotator (Math|Rotator|FindLookatRotation (CallFunction|GetEffectLocation) (CallFunction|GetTargetLocation)))))) "AdjustIfPossibleButAlwaysSpawn" "SelectDefaultAtRuntime" (Variables|Default|GetOwnerCharacter) 0))
  (Utilities|IsValid _returnvalue
    (:Is%20Valid
      (Default|SetTargetActor (Variables|/Game/DynamicCombatSystem/DCS/Blueprints/AI/BP_BaseAI.BP_BaseAI_C|GetBaseAIController _returnvalue) (CallFunction|GetTarget))
      (Default|AddActivityforDuration (Variables|/Game/DynamicCombatSystem/DCS/Blueprints/AI/BP_BaseAI.BP_BaseAI_C|GetStateManager _returnvalue) "(TagName=\"Activity.IsMarkedToKill\")" false (Variables|Ability|Custom|GetLifeTime) false) ; Adding activity to spawned AI\nwhen it end, AI will die
    )))