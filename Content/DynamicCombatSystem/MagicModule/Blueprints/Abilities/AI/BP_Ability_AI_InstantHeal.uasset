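; AI magic ability that instantly heals the casting character.
; On release, it asks the AbilityComponent to start casting and, if allowed, plays the ability montage.
; When the effect event fires, it raises the owner's current health stat through the StatsManager by HealAmount, attaches a heal sound and particle to the character mesh, then applies the ability cost.
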(event Custom|SpawnParticle
  ;[0 0.272 1] Spawn heal particle
  (Effects|SpawnEmitterAttached (Variables|Ability|Cusotm|GetHealParticle) (Variables|/Script/Engine.Character|GetMesh (Variables|Default|GetOwnerCharacter)) "" "0, 0,20.000000"))

(event Custom|PlaySound
  ;[0 0.272 1] Play Sound
  (Audio|SpawnSoundAttached (Variables|Ability|Cusotm|GetSound) (Variables|/Script/Engine.Character|GetMesh (Variables|Default|GetOwnerCharacter)) "None" "0, 0, 0" "0, 0, 0" "KeepRelativeOffset" false 1.0 1.0 0.0 0 0))

(event EventdReleased
  ;[0 0.272 1] On released check whether ability can be started and play montage
  (bind _result (Default|StartCastingAbility (Variables|Default|GetAbilityComponent)))
  (if _result
    (CallFunction|PlayAbilityMontage (CallFunction|GetAbilityMontage) "None" -1.0)))

(event EventdSpawnEffect
  ;[0 0.272 1] On effect heal owner
  (CallFunction|Heal)
  (CallFunction|PlaySound)
  (CallFunction|SpawnParticle)
  (CallFunction|ApplyAbilityCost -1.0 1.0))

(fn ConstructionScript
  (|CallParentFunction))

(fn Heal
  (Default|ModifyStat (Variables|/Game/DynamicCombatSystem/DCS/Blueprints/AI/BP_BaseAI.BP_BaseAI_C|GetStatsManager (Variables|Default|GetAICharacter)) "(TagName=\"Stat.Health.Current\")" (Variables|Ability|Cusotm|GetHealAmount)))