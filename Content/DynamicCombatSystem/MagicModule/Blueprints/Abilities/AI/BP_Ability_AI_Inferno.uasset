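; AI Inferno ability from the magic module that casts a delayed area-damage effect at a predicted target position.
; On release it starts casting, plays the montage, stores a surface-projected predicted target transform within range and shows an indicator there.
; The effect event spawns a damage sphere actor at that stored transform with the ability's radius and damage, adds particle and sound, then applies the ability cost.
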(event Custom|SpawnParticle
  ;[0 0.272 1] Spawn Particle
  (Effects|SpawnEmitteratLocation (Variables|Ability|Custom|GetHitParticle) (CallFunction|GetEffectLocation)))

(event Custom|PlaySound
  ;[0 0.272 1] Play Sound
  (Audio|PlaySoundatLocation (Variables|Ability|Custom|GetSound) (CallFunction|GetEffectLocation) "0, 0, 0" 1.0 1.0 0.0 0 0 0 0))

(event EventdReleased
  ;[0 0.272 1] On Pressed play anim montage, update effect transform and show indicator
  (bind _result (Default|StartCastingAbility (Variables|Default|GetAbilityComponent)))
  (if _result
    (CallFunction|PlayAbilityMontage (CallFunction|GetAbilityMontage) "None" -1.0)
    (bind _result_2 (CallFunction|GetSurfacePredictedTargetTransform (Variables|Ability|Custom|GetRange)))
    (Variables|Default|SetEffectTransform _result_2)
    (CallFunction|ShowIndicator (CallFunction|GetEffectLocation))))

(event EventdSpawnEffect
  (bind _returnvalue (Components|GetOwner))
  ;[0 0.272 1] On effect spawn damage sphere
  (Game|SpawnActorfromClass "/Game/DynamicCombatSystem/DCS/Blueprints/Components/Ability/AbilityEffects/BP_AE_DamageSphere.BP_AE_DamageSphere_C" (Variables|Default|GetEffectTransform) "AlwaysSpawn" "OverrideRootScale" _returnvalue (Variables|Ability|Custom|GetRadius) (CallFunction|GetDamage 1.0) "None" (Game|GetInstigator _returnvalue))
  (CallFunction|SpawnParticle)
  (CallFunction|PlaySound)
  (CallFunction|ApplyAbilityCost -1.0 1.0))

(fn ConstructionScript
  (|CallParentFunction))