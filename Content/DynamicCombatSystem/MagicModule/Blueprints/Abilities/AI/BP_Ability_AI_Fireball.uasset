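; AI fireball ability in the Dynamic Combat System magic module that launches a damaging projectile, homing on the target when valid.
; Release plays a cast montage, opening with the first then alternating the next two during continued casting, with a retriggerable delay resetting the chain.
; A looping timer, used instead of tick, aims the effect transform from the montage's casting hand toward the target.
; The effect event spawns the projectile, stops the timer and applies the cost.
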(event Custom|ResetMontageCounter
  ;[0 0.272 1] When casted first, use montage at index 0 and then if keeps casting, use montages at indexes 1 & 2
  (Variables|NonEdit|SetMontageCounter 0))

(event Custom|UpdateMontageCounter
  ;[0 0.272 1] When casted first, use montage at index 0 and then if keeps casting, use montages at indexes 1 & 2
  (bind _result (Math|Integer|IncrementInt (Variables|NonEdit|GetMontageCounter))
    (:%20%20
      (if (> _result (Utilities|Array|LastIndex (Variables|Default|GetAbilityMontages)))
        (Variables|NonEdit|SetMontageCounter 1)))))

(event Custom|UpdateSocket
  ;[0 0.272 1] Use left hand socket only for 1st index because animation at this index uses left hand
  (switch int (Variables|NonEdit|GetMontageCounter)
    (:0
      (Variables|NonEdit|SetUseLeftHandSocket false))
    (:1
      (Variables|NonEdit|SetUseLeftHandSocket true))
    (:2
      (Variables|NonEdit|SetUseLeftHandSocket false))))

(event Custom|UpdateEffect
  (bind _targetlocation (CallFunction|GetTargetLocation))
  (bind _lefthandsocket (Variables|Default|GetLeftHandSocket))
  (bind _righthandsocket (Variables|Default|GetRightHandSocket))
  (bind _uselefthandsocket (Variables|NonEdit|GetUseLeftHandSocket))
  (bind _returnvalue (select _uselefthandsocket _lefthandsocket _righthandsocket))
  (bind _socketlocation (CallFunction|GetSocketLocationonOwnerMesh _returnvalue))
  (bind _returnvalue_2 (Math|Rotator|FindLookatRotation _socketlocation _targetlocation))
  ;[0 0.272 1] Update effect transform
  (Variables|Default|SetEffectTransform (Math|Transform|MakeTransform (+ _socketlocation (Math|Rotator|GetRotationXVector _returnvalue_2)) _returnvalue_2)))

(event Custom|StartTimer
  ;[0 0.272 1] Use timer updating ability effect instead of doing it on tick
  (Utilities|Time|SetTimerbyEvent (EventDispatchers|CreateEvent :!event Custom|UpdateEffect) 0.016 true))

(event Custom|StopTimer
  ;[0 0.272 1] Use timer updating ability effect instead of doing it on tick
  (Utilities|Time|ClearTimerbyFunctionName 0 "UpdateEffect"))

(event EventdFinished
  (params (Result :type E_AbilityFinishResult%20Enum :default "NewEnumerator0"))
  ;[0 0.272 1] Stop timer updating effect when ability ends
  (CallFunction|StopTimer))

(event EventdReleased
  ;[0 0.272 1] On released check whether ability can be started and update montage index and play it
  (bind _result (Default|StartCastingAbility (Variables|Default|GetAbilityComponent)))
  (if _result
    (CallFunction|StartTimer)
    (CallFunction|UpdateSocket)
    (bind _duration (CallFunction|PlayAbilityMontage (CallFunction|GetAbilityMontage (Variables|NonEdit|GetMontageCounter)) "None" -1.0))
    (CallFunction|UpdateMontageCounter)
    (Utilities|FlowControl|RetriggerableDelay _duration)
    (CallFunction|ResetMontageCounter)))

(event EventdSpawnEffect
  (bind _target (CallFunction|GetTarget))
  (bind _returnvalue (Components|GetOwner))
  (bind _returnvalue_2 (Game|GetInstigator _returnvalue))
  ;[0 0.272 1] On effect spawn homing projectile
  (CallFunction|UpdateEffect)
  (bind _returnvalue_3 (Game|SpawnActorfromClass "/Game/DynamicCombatSystem/MagicModule/Blueprints/Projectiles/Instances/BP_MovingProjectile_Fireball.BP_MovingProjectile_Fireball_C" (Variables|Default|GetEffectTransform) "AlwaysSpawn" "OverrideRootScale" _returnvalue_2 (Variables|Default|GetDamage) 1.5e+03 1e+04 true _returnvalue_2))
  (Utilities|FlowControl|Sequence
    (:then_0
      (Utilities|IsValid _target
        (:Is%20Valid
          (Default|StartHoming _returnvalue_3 (Variables|/Script/Engine.Actor|GetRootComponent _target) 3e+02))))
    (:then_1
      (CallFunction|StopTimer)
      (CallFunction|ApplyAbilityCost -1.0 1.0))))

(fn ConstructionScript
  (|CallParentFunction))