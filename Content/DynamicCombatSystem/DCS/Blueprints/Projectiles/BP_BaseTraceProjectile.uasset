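; Base hitscan-style projectile for the combat system that resolves its hit with an instant trace when started.
; StartProjectile runs a multi sphere trace along the actor's forward vector up to MaxRange, ignoring the owner, and takes the first hit.
; The result feeds SpawnTracerEffect, an empty hook presumably for child classes, then a hit goes to HandleHit while a miss destroys the actor.
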(event EventStartProjectile
  (bind (_washit _hitresult) (CallFunction|DoProjectileTraceTest))
  (CallFunction|SpawnTracerEffect _hitresult)
  (if _washit
    (CallFunction|HandleHit _hitresult)
    (else
      (Actor|DestroyActor))))

(fn ConstructionScript
  (|CallParentFunction))

(fn DoProjectileTraceTest
  (bind _returnvalue (Transformation|GetActorLocation))
  (bind _outhits (Collision|MultiSphereTraceByChannel _returnvalue (+ _returnvalue (* (Transformation|GetActorForwardVector) (Variables|Default|GetMaxRange))) (Variables|Default|GetTraceRadius) (CallFunction|GetProjectileChannel) false (Utilities|Array|MakeArray (Components|GetOwner)) (select (Variables|Default|GetDebug) "ForDuration" "None") true "(R=1.000000,G=0.000000,B=0.000000,A=1.000000)" "(R=0.000000,G=1.000000,B=0.000000,A=1.000000)" 2.0))
  (for _array_element _outhits
    ;[1 1 1] each actor can be checked only once
    (bind _returnvalue_2 (Utilities|Array|AddUnique (LocalVariables|GetL_HitActors) (.HitActor (Collision|BreakHitResult _array_element))))
    (if (>= _returnvalue_2 0)
      (return true _array_element)))
  (return false ""))

(fn SpawnTracerEffect
  (params (HitResult :type Hit%20Result%20Structure%20%28by%20ref%29)))