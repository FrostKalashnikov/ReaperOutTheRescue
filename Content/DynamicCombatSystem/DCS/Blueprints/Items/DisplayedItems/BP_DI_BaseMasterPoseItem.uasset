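; BP_DI_BaseMasterPoseItem is a displayed-item base in the Dynamic Combat System for items whose skeletal meshes follow the owning character's animation.
; It overrides Attach, running the parent attachment first, then using Set Leader Pose Component to slave its skeletal mesh to the owner Character's Mesh.
; The return sits inside the component loop, so only the first skeletal mesh component found is linked.
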(event EventBeginPlay
  (|CallParentFunction) ; This node is disabled and will not be called.\nDrag off pins to build functionality.
)

(event Collision|EventActorBeginOverlap
  (params (OtherActor :type Actor%20Object%20Reference)))

(event EventTick
  (params (DeltaSeconds :type Float%20%28single-precision%29)))

(fn ConstructionScript
  (|CallParentFunction))

(fn Attach
  (bind _result (|CallParentFunction))
  (if _result
    (for _array_element (Actor|GetComponentsByClass "/Script/Engine.SkeletalMeshComponent")
      (Components|SkinnedMesh|SetLeaderPoseComponent _array_element (Variables|/Script/Engine.Character|GetMesh (.AsCharacter (Utilities|Casting|CastToCharacter (Components|GetOwner)))) false false)
      (return true))))