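; BP_DA_Item_MeleeWeapon is the Dynamic Combat System item definition for a melee weapon.
; It exposes the weapon's ability, block value, displayed item, stat modifiers and two-handed flag through simple getter functions.
; Each getter returns its stored variable directly, with no further logic in the asset.
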(fn GetAbility
  (return (Variables|Ability|GetAbility)))

(fn GetBlockValue
  (return (Variables|Weapon|GetBlockValue)))

(fn GetDisplayedItem
  (return (Variables|Display|GetDisplayedItem)))

(fn GetModifiers
  (return (Variables|Modifiers|GetModifiers)))

(fn IsTwoHanded
  (return (Variables|Weapon|GetTwoHanded)))