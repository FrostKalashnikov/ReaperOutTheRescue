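; Actor component in the Dynamic Combat System that manages its owner's movement speed state (idle, walk, jog, sprint).
; On BeginPlay it caches the owner's CharacterMovementComponent and applies the default state.
; A state change sets the max walk and crouched speeds from configured values and notifies listeners with previous and new states.
; An optional debug tick prints the current state and speed.
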(event EventBeginPlay
  (CallFunction|Initialize)
  (if (Variables|Settings|GetDebug)
    (Components|Tick|SetComponentTickEnabled true)))

(event EventTick
  (params (DeltaSeconds :type Float%20%28single-precision%29))
  (if (Variables|Settings|GetDebug)
    (CallFunction|DebugTick DeltaSeconds)))

(fn GetMovementState
  (return (Variables|Default|GetMovementState)))

(fn SetMovementState
  (params (State :type E_MovementState%20Enum :default "NewEnumerator0"))
  (bind _ownercharactermovementcomp (Variables|Default|GetOwnerCharacterMovementComp))
  (if (Utilities|Enum|NotEqual(Enum) State (Variables|Default|GetMovementState))
    (LocalVariables|SetL_PreviousMoveSpeed (Variables|Default|GetMovementState))
    (Variables|Default|SetMovementState State)
    (Variables|/Script/Engine.CharacterMovementComponent|SetMaxWalkSpeed _ownercharactermovementcomp (Utilities|Select :Index (Variables|Default|GetMovementState) :NewEnumerator0 0.0 :NewEnumerator1 (Variables|Settings|GetWalkSpeed) :NewEnumerator2 (Variables|Settings|GetJogSpeed) :NewEnumerator3 (Variables|Settings|GetSprintSpeed)))
    (Variables|/Script/Engine.CharacterMovementComponent|SetMaxWalkSpeedCrouched _ownercharactermovementcomp (Variables|Settings|GetCrouchSpeed))
    (Default|CallOnMovementSpeedChanged (LocalVariables|GetL_PreviousMoveSpeed) (Variables|Default|GetMovementState))))

(fn DebugTick
  (params (DeltaTime :type Float%20%28double-precision%29))
  (Development|PrintText (Utilities|Text|FormatText "{owner}: Move Speed: {mode} - {speed}" (Components|GetOwner) (Utilities|String|EnumtoString (Variables|Default|GetMovementState)) (Class|MovementComponent|GetMaxSpeed (Variables|Default|GetOwnerCharacterMovementComp))) true false "(R=0.431254,G=0.000000,B=1.000000,A=1.000000)" DeltaTime))

(fn Initialize
  (Utilities|FlowControl|Sequence
    (:then_0
      (Variables|Default|SetOwnerCharacterMovementComp (Actor|GetComponentbyClass (Components|GetOwner) "/Script/Engine.CharacterMovementComponent")))
    (:then_1
      (Interface|SetMovementState (Variables|Settings|GetDefaultMovementState)))))

(fn IsMovementState
  (params (StateToCheck :type E_MovementState%20Enum :default "NewEnumerator0"))
  (return (Utilities|Enum|Equal(Enum) StateToCheck (Interface|GetMovementState))))