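; BP_DCSGameMode is the Dynamic Combat System game mode that handles saving and loading a player's game.
; SaveGame creates a BP_DCSSaveGame object if none exists, has it capture the player's data, then writes it asynchronously to a named slot.
; LoadGame reads that slot asynchronously, caches the save object and has it apply its data to the player, with a printed confirmation.
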(event Custom|SaveGame
  (params (Player :type Actor%20Object%20Reference))
  ;[1 0 0] Save / Load Game
  (Variables|Default|GetDCSSaveGame
    (:then
      _)
    (:else
      (bind _returnvalue (SaveGame|CreateSaveGameObject "/Game/DynamicCombatSystem/DCS/Blueprints/BP_DCSSaveGame.BP_DCSSaveGame_C"))
      (Variables|Default|SetDCSSaveGame _returnvalue)))
  (Default|SaveData (Variables|Default|GetDCSSaveGame) Player)
  (bind _bsuccess (|AsyncSaveGametoSlot (Variables|Default|GetDCSSaveGame) (Variables|Default|GetSaveSlotName))
    (:Completed
      (if _bsuccess
        (Development|PrintString "DCS Game Saved" true true "(R=1.000000,G=0.000000,B=0.627968,A=1.000000)" 5.0)))))

(event Custom|LoadGame
  (params (Player :type Actor%20Object%20Reference))
  ;[1 0 0] Save / Load Game
  (bind _savegame (|AsyncLoadGamefromSlot (Variables|Default|GetSaveSlotName))
    (:Completed
      (bind _asbp_dcssave_game (Utilities|Casting|CastToBP_DCSSaveGame _savegame))
      (bind _output_get (Variables|Default|SetDCSSaveGame _asbp_dcssave_game))
      (Default|LoadData _output_get Player)
      (Development|PrintString "DCS Game Loaded" true true "(R=1.000000,G=0.000000,B=0.627968,A=1.000000)" 5.0))))

(fn ConstructionScript)